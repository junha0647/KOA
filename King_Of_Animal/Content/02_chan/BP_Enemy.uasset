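; BP_Enemy relays second-player input for what appears to be a two-player fighting game.
; Its P2 action events for jump press and release, left and right punches and left and right kicks call matching functions on an Opponent reference.
; The MoveRight_P2 axis passes its value through the same way.
; It holds no combat logic of its own, and nothing here assigns Opponent.
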(event EventBeginPlay
  (|CallParentFunction) ; 지금 이 노드는 비활성 상태입니다. \n핀을 끌어서 다른 노드를 연결하면 활성화됩니다.
)

(event Collision|EventActorBeginOverlap
  (params (OtherActor :type Actor%20Object%20Reference))
  (|CallParentFunction OtherActor) ; 지금 이 노드는 비활성 상태입니다. \n핀을 끌어서 다른 노드를 연결하면 활성화됩니다.
)

(event EventTick
  (params (DeltaSeconds :type Float%20%28single-precision%29))
  (|CallParentFunction DeltaSeconds) ; 지금 이 노드는 비활성 상태입니다. \n핀을 끌어서 다른 노드를 연결하면 활성화됩니다.
)

(event Input|ActionEvents|InputActionJumpP2
  (params (Key :type Key%20Structure :default "None"))
  (bind _opponent (Variables|Default|Getopponent))
  (:Pressed
    (Class|CPPCharacter|JumpP2 _opponent))
  (:Released
    (Class|CPPCharacter|StopJumpP2 _opponent)))

(event Input|ActionEvents|InputActionL_Punch_P2
  (params (Key :type Key%20Structure :default "None"))
  (:Pressed
    (Class|CPPCharacter|LPunchP2 (Variables|Default|Getopponent))))

(event Input|ActionEvents|InputActionR_Punch_P2
  (params (Key :type Key%20Structure :default "None"))
  (:Pressed
    (Class|CPPCharacter|RPunchP2 (Variables|Default|Getopponent))))

(event Input|ActionEvents|InputActionL_Kick_P2
  (params (Key :type Key%20Structure :default "None"))
  (:Pressed
    (Class|CPPCharacter|LKickP2 (Variables|Default|Getopponent))))

(event Input|ActionEvents|InputActionR_Kick_P2
  (params (Key :type Key%20Structure :default "None"))
  (:Pressed
    (Class|CPPCharacter|RKickP2 (Variables|Default|Getopponent))))

(event Input|AxisEvents|InputAxisMoveRight_P2
  (params (AxisValue :type Float%20%28single-precision%29))
  (Class|CPPCharacter|MoveRightP2 (Variables|Default|Getopponent) AxisValue))

(fn ConstructionScript
  (|CallParentFunction))