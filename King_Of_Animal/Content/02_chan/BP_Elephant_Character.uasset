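; Elephant character for the King of Animal fighting game that relays player two's input and opens the pause menu.
; On BeginPlay it caches Player2 from the game mode, then forwards P2 jump, crouch, movement, punch, kick, uppercut and exceptional attack actions to it.
; A P1 action records timestamped keys in an input buffer, pruning stale entries and printing the contents for debugging.
; Q or Escape shows the pause widget with UI-only input.
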(event EventBeginPlay
  (bind _asking_of_animal_game_mode (Utilities|Casting|CastToKing_Of_AnimalGameMode (Game|GetGameMode)))
  (Utilities|IsValid (Variables|/Script/King_Of_Animal.King_Of_AnimalGameMode|Getplayer2 _asking_of_animal_game_mode)
    (:Is%20Valid
      (Variables|Default|SetPlayer%202%20Reference (Variables|/Script/King_Of_Animal.King_Of_AnimalGameMode|Getplayer2 _asking_of_animal_game_mode)))))

(event Input|ActionEvents|InputActionJumpP2
  (params (Key :type Key%20Structure :default "None"))
  (bind _player_2_reference (Variables|Default|GetPlayer%202%20Reference))
  (bind _player_2_reference_2 (Variables|Default|GetPlayer%202%20Reference))
  (:Pressed
    (Utilities|IsValid _player_2_reference_2
      (:Is%20Valid
        (Class|CPPCharacter|JumpP2 _player_2_reference_2))))
  (:Released
    (Utilities|IsValid _player_2_reference
      (:Is%20Valid
        (Class|CPPCharacter|StopJumpP2 _player_2_reference)))))

(event Input|ActionEvents|InputActionL_Punch_P2
  (params (Key :type Key%20Structure :default "None"))
  (bind _player_2_reference (Variables|Default|GetPlayer%202%20Reference))
  (:Pressed
    (Utilities|IsValid _player_2_reference
      (:Is%20Valid
        (Class|CPPCharacter|LPunchP2 _player_2_reference)))))

(event Input|ActionEvents|InputActionR_Punch_P2
  (params (Key :type Key%20Structure :default "None"))
  (bind _player_2_reference (Variables|Default|GetPlayer%202%20Reference))
  (:Pressed
    (Utilities|IsValid _player_2_reference
      (:Is%20Valid
        (Class|CPPCharacter|RPunchP2 _player_2_reference)))))

(event Input|ActionEvents|InputActionL_Kick_P2
  (params (Key :type Key%20Structure :default "None"))
  (bind _player_2_reference (Variables|Default|GetPlayer%202%20Reference))
  (:Pressed
    (Utilities|IsValid _player_2_reference
      (:Is%20Valid
        (Class|CPPCharacter|LKickP2 _player_2_reference)))))

(event Input|ActionEvents|InputActionR_Kick_P2
  (params (Key :type Key%20Structure :default "None"))
  (bind _player_2_reference (Variables|Default|GetPlayer%202%20Reference))
  (:Pressed
    (Utilities|IsValid _player_2_reference
      (:Is%20Valid
        (Class|CPPCharacter|RKickP2 _player_2_reference)))))

(event Input|ActionEvents|InputActionCrouch_P2
  (params (Key :type Key%20Structure :default "None"))
  (bind _player_2_reference (Variables|Default|GetPlayer%202%20Reference))
  (bind _player_2_reference_2 (Variables|Default|GetPlayer%202%20Reference))
  (:Pressed
    (Utilities|IsValid _player_2_reference
      (:Is%20Valid
        (Class|CPPCharacter|StartCrouching _player_2_reference))))
  (:Released
    (Utilities|IsValid _player_2_reference_2
      (:Is%20Valid
        (Class|CPPCharacter|StopCrouching _player_2_reference_2)))))

(event Input|ActionEvents|InputActionUppercut_P2
  (params (Key :type Key%20Structure :default "None"))
  (bind _player_2_reference (Variables|Default|GetPlayer%202%20Reference))
  (:Pressed
    (Utilities|IsValid _player_2_reference
      (:Is%20Valid
        (Class|CPPCharacter|UppercutP2 _player_2_reference)))))

(event Input|ActionEvents|InputActionExceptionalAttack_P2
  (params (Key :type Key%20Structure :default "None"))
  (bind _player_2_reference (Variables|Default|GetPlayer%202%20Reference))
  (:Pressed
    (Utilities|IsValid _player_2_reference
      (:Is%20Valid
        (Class|CPPCharacter|StartExceptionalAttackP2 _player_2_reference)))))

(event Input|ActionEvents|InputActionAddToInputBuffer_P1
  (params (Key :type Key%20Structure :default "None"))
  (bind _inputbuffer (Variables|Default|GetinputBuffer))
  (:Pressed
    (for _array_element _inputbuffer
      (if (< (.timeStamp (Utilities|Struct|BreakInputInfo _array_element)) (- (Utilities|Time|GetTimeSeconds) 0.2))
        (Utilities|Array|RemoveItem _inputbuffer _array_element)))
    (Class|CPPCharacter|AddInputtoInputBuffer (Utilities|Struct|MakeInputInfo (Utilities|String|ToString(Text) (Class|KismetInputLibrary|KeyGetDisplayName Key)) (Utilities|Time|GetTimeSeconds)))
    ;[1 1 1] Showcase what elements in the input buffer
    (for _array_element_2 (Variables|Default|GetinputBuffer)
      (Development|PrintString (.inputName (Utilities|Struct|BreakInputInfo _array_element_2))))))

(event Input|AxisEvents|InputAxisMoveRight_P2
  (params (AxisValue :type Float%20%28single-precision%29))
  (bind _player_2_reference (Variables|Default|GetPlayer%202%20Reference))
  (Utilities|IsValid _player_2_reference
    (:Is%20Valid
      (Class|CPPCharacter|MoveRightP2 _player_2_reference AxisValue))))

(event Input|KeyboardEvents|Escape
  (params (Key :type Key%20Structure :default "None"))
  (bind _returnvalue (Game|GetPlayerController 0))
  ;[1 1 1] Pause Menu
  (:Pressed
    (Utilities|IsValid (Variables|Default|GetPause%20Reference)
      (:Is%20Valid
        _)
      (:Is%20Not%20Valid
        (bind _returnvalue_2 (UserInterface|CreateWidget "/Game/03_su/WidgetBP/Pause.Pause_C"))
        (Variables|Default|SetPause%20Reference _returnvalue_2)))
    (Variables|/Script/Engine.PlayerController|SetbShowMouseCursor _returnvalue true)
    (Input|SetInputModeUIOnly _returnvalue (Variables|Default|GetPause%20Reference) "DoNotLock")
    (UserInterface|Viewport|AddtoViewport (Variables|Default|GetPause%20Reference) 0)))

(event Input|KeyboardEvents|Q
  (params (Key :type Key%20Structure :default "None"))
  (bind _returnvalue (Game|GetPlayerController 0))
  ;[1 1 1] Pause Menu
  (:Pressed
    (Utilities|IsValid (Variables|Default|GetPause%20Reference)
      (:Is%20Valid
        _)
      (:Is%20Not%20Valid
        (bind _returnvalue_2 (UserInterface|CreateWidget "/Game/03_su/WidgetBP/Pause.Pause_C"))
        (Variables|Default|SetPause%20Reference _returnvalue_2)))
    (Variables|/Script/Engine.PlayerController|SetbShowMouseCursor _returnvalue true)
    (Input|SetInputModeUIOnly _returnvalue (Variables|Default|GetPause%20Reference) "DoNotLock")
    (UserInterface|Viewport|AddtoViewport (Variables|Default|GetPause%20Reference) 0)))

(fn ConstructionScript)