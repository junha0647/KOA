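; BP_Character is a character Blueprint that relays player-two fighting controls to an Opponent reference and puts the health UI on screen.
; On BeginPlay it creates a WBP_Health widget and adds it to the viewport.
; Its P2 input events for movement, jump press and release, punches and kicks call matching functions on Opponent, so this Blueprint receives the input while Opponent carries out the actions.
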(event EventBeginPlay
  (bind _returnvalue (UserInterface|CreateWidget "/Game/03_su/WBP_Health.WBP_Health_C"))
  (UserInterface|Viewport|AddtoViewport _returnvalue 0))

(event Collision|EventActorBeginOverlap
  (params (OtherActor :type Actor%20Object%20Reference)))

(event EventTick
  (params (DeltaSeconds :type Float%20%28single-precision%29)))

(event Input|ActionEvents|InputActionJumpP2
  (params (Key :type Key%20Structure :default "None"))
  (bind _opponent (Variables|Default|Getopponent))
  (:Pressed
    (Class|CPPCharacter|JumpP2 _opponent))
  (:Released
    (Class|CPPCharacter|StopJumpP2 _opponent)))

(event Input|ActionEvents|InputActionL_Punch_P2
  (params (Key :type Key%20Structure :default "None"))
  (:Pressed
    (Class|CPPCharacter|LPunchP2 (Variables|Default|Getopponent))))

(event Input|ActionEvents|InputActionR_Punch_P2
  (params (Key :type Key%20Structure :default "None"))
  (:Pressed
    (Class|CPPCharacter|RPunchP2 (Variables|Default|Getopponent))))

(event Input|ActionEvents|InputActionL_Kick_P2
  (params (Key :type Key%20Structure :default "None"))
  (:Pressed
    (Class|CPPCharacter|LKickP2 (Variables|Default|Getopponent))))

(event Input|ActionEvents|InputActionR_Kick_P2
  (params (Key :type Key%20Structure :default "None"))
  (:Pressed
    (Class|CPPCharacter|RKickP2 (Variables|Default|Getopponent))))

(event Input|AxisEvents|InputAxisMoveRight_P2
  (params (AxisValue :type Float%20%28single-precision%29))
  (Class|CPPCharacter|MoveRightP2 (Variables|Default|Getopponent) AxisValue))

(fn ConstructionScript)