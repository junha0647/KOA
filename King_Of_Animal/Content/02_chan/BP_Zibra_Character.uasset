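; Zebra fighter character for a local two-player fighting game that also relays Player 2's moves, attacks and skills to the game mode's Player2 character.
; Q or Escape opens the pause menu.
; On player lock-in, it scans project input mappings to build key-to-input-type maps for both players and adds per-player buffer actions at runtime.
; Those actions append timestamped inputs to each player's buffer, pruning entries older than 0.2 seconds.
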(event EventBeginPlay
  (bind _asking_of_animal_game_mode (Utilities|Casting|CastToKing_Of_AnimalGameMode (Game|GetGameMode)))
  (Utilities|IsValid (Variables|/Script/King_Of_Animal.King_Of_AnimalGameMode|Getplayer2 _asking_of_animal_game_mode)
    (:Is%20Valid
      (Variables|Default|SetPlayer2%20Reference (Variables|/Script/King_Of_Animal.King_Of_AnimalGameMode|Getplayer2 _asking_of_animal_game_mode)))))

(event EventNotifyPlayerLockedin
  (CallFunction|SetUpInputMappings))

(event Input|ActionEvents|InputActionJumpP2
  (params (Key :type Key%20Structure :default "None"))
  (bind _player2_reference (Variables|Default|GetPlayer2%20Reference))
  (bind _player2_reference_2 (Variables|Default|GetPlayer2%20Reference))
  (:Pressed
    (Utilities|IsValid _player2_reference
      (:Is%20Valid
        (Class|CPPCharacter|JumpP2 _player2_reference))))
  (:Released
    (Utilities|IsValid _player2_reference_2
      (:Is%20Valid
        (Class|CPPCharacter|StopJumpP2 _player2_reference_2)))))

(event Input|ActionEvents|InputActionL_Punch_P2
  (params (Key :type Key%20Structure :default "None"))
  (bind _player2_reference (Variables|Default|GetPlayer2%20Reference))
  (:Pressed
    (Utilities|IsValid _player2_reference
      (:Is%20Valid
        (Class|CPPCharacter|LPunchP2 _player2_reference)))))

(event Input|ActionEvents|InputActionSkill_2_P2
  (params (Key :type Key%20Structure :default "None"))
  (bind _player2_reference (Variables|Default|GetPlayer2%20Reference))
  (:Pressed
    (Utilities|IsValid _player2_reference
      (:Is%20Valid
        (Class|CPPCharacter|Skill2P2 _player2_reference)))))

(event Input|ActionEvents|InputActionSkill_Ult_P2
  (params (Key :type Key%20Structure :default "None"))
  (bind _player2_reference (Variables|Default|GetPlayer2%20Reference))
  (:Pressed
    (Utilities|IsValid _player2_reference
      (:Is%20Valid
        (Class|CPPCharacter|SkillUltP2 _player2_reference)))))

(event Input|ActionEvents|InputActionR_Punch_P2
  (params (Key :type Key%20Structure :default "None"))
  (bind _player2_reference (Variables|Default|GetPlayer2%20Reference))
  (:Pressed
    (Utilities|IsValid _player2_reference
      (:Is%20Valid
        (Class|CPPCharacter|RPunchP2 _player2_reference)))))

(event Input|ActionEvents|InputActionL_Kick_P2
  (params (Key :type Key%20Structure :default "None"))
  (bind _player2_reference (Variables|Default|GetPlayer2%20Reference))
  (:Pressed
    (Utilities|IsValid _player2_reference
      (:Is%20Valid
        (Class|CPPCharacter|LKickP2 _player2_reference)))))

(event Input|ActionEvents|InputActionR_Kick_P2
  (params (Key :type Key%20Structure :default "None"))
  (bind _player2_reference (Variables|Default|GetPlayer2%20Reference))
  (:Pressed
    (Utilities|IsValid _player2_reference
      (:Is%20Valid
        (Class|CPPCharacter|RKickP2 _player2_reference)))))

(event Input|ActionEvents|InputActionCrouch_P2
  (params (Key :type Key%20Structure :default "None"))
  (bind _player2_reference (Variables|Default|GetPlayer2%20Reference))
  (bind _player2_reference_2 (Variables|Default|GetPlayer2%20Reference))
  (:Pressed
    (Utilities|IsValid _player2_reference
      (:Is%20Valid
        (Class|CPPCharacter|StartCrouching _player2_reference))))
  (:Released
    (Utilities|IsValid _player2_reference_2
      (:Is%20Valid
        (Class|CPPCharacter|StopCrouching _player2_reference_2)))))

(event Input|ActionEvents|InputActionSkill_1_P2
  (params (Key :type Key%20Structure :default "None"))
  (bind _player2_reference (Variables|Default|GetPlayer2%20Reference))
  (:Pressed
    (Utilities|IsValid _player2_reference
      (:Is%20Valid
        (Class|CPPCharacter|Skill1P2 _player2_reference)))))

(event Input|ActionEvents|InputActionAddToInputBuffer_P1
  (params (Key :type Key%20Structure :default "None"))
  (bind _returnvalue (Class|KismetInputLibrary|KeyGetDisplayName Key))
  (bind _inputbuffer (Variables|Default|GetinputBuffer))
  (bind _inputtoinputtypemap (Variables|Default|GetinputToInputTypeMap))
  (bind _returnvalue_2 (Utilities|String|ToString(Text) _returnvalue))
  (bind _value (Utilities|Map|Find _inputtoinputtypemap _returnvalue_2))
  (:Pressed
    (for _array_element _inputbuffer
      (if (< (.timeStamp (Utilities|Struct|BreakInputInfo _array_element)) (- (Utilities|Time|GetTimeSeconds) 0.2))
        (Utilities|Array|RemoveItem _inputbuffer _array_element)))
    (Class|CPPCharacter|AddInputtoInputBuffer (Utilities|Struct|MakeInputInfo _value _returnvalue_2 (Utilities|Time|GetTimeSeconds) false))
    (Development|PrintString (Utilities|String|ToString(Name) (Utilities|Name|EnumtoName _value)))))

(event Input|ActionEvents|InputActionAddToInputBuffer_P2
  (params (Key :type Key%20Structure :default "None"))
  (bind _returnvalue (Class|KismetInputLibrary|KeyGetDisplayName Key))
  (bind _player2_reference (Variables|Default|GetPlayer2%20Reference))
  (bind _returnvalue_2 (Utilities|String|ToString(Text) _returnvalue))
  (:Pressed
    (bind _player2_reference_2 (Variables|Default|GetPlayer2%20Reference)
      (:then
        (for _array_element (Variables|/Script/King_Of_Animal.CPP_Character|GetinputBuffer _player2_reference_2)
          (if (< (.timeStamp (Utilities|Struct|BreakInputInfo _array_element)) (- (Utilities|Time|GetTimeSeconds) 0.2))
            (Utilities|Array|RemoveItem (Variables|/Script/King_Of_Animal.CPP_Character|GetinputBuffer _player2_reference_2) _array_element)))
        (Class|CPPCharacter|AddInputtoInputBuffer _player2_reference (Utilities|Struct|MakeInputInfo (.Value (Utilities|Map|Find (Variables|/Script/King_Of_Animal.CPP_Character|GetinputToInputTypeMap _player2_reference) _returnvalue_2)) _returnvalue_2 (Utilities|Time|GetTimeSeconds) false)))
      (:else))))

(event Input|AxisEvents|InputAxisMoveRight_P2
  (params (AxisValue :type Float%20%28single-precision%29))
  (bind _player2_reference (Variables|Default|GetPlayer2%20Reference))
  (Utilities|IsValid _player2_reference
    (:Is%20Valid
      (Class|CPPCharacter|MoveRightP2 _player2_reference AxisValue))))

(event Input|KeyboardEvents|Escape
  (params (Key :type Key%20Structure :default "None"))
  (bind _returnvalue (Game|GetPlayerController 0))
  ;[1 1 1] Pause Menu
  (:Pressed
    (Utilities|IsValid (Variables|Default|GetPause%20Reference)
      (:Is%20Valid
        _)
      (:Is%20Not%20Valid
        (bind _returnvalue_2 (UserInterface|CreateWidget "/Game/03_su/WidgetBP/Pause.Pause_C"))
        (Variables|Default|SetPause%20Reference _returnvalue_2)))
    (Variables|/Script/Engine.PlayerController|SetbShowMouseCursor _returnvalue true)
    (Input|SetInputModeUIOnly _returnvalue (Variables|Default|GetPause%20Reference) "DoNotLock")
    (UserInterface|Viewport|AddtoViewport (Variables|Default|GetPause%20Reference) 0)))

(event Input|KeyboardEvents|Q
  (params (Key :type Key%20Structure :default "None"))
  (bind _returnvalue (Game|GetPlayerController 0))
  ;[1 1 1] Pause Menu
  (:Pressed
    (Utilities|IsValid (Variables|Default|GetPause%20Reference)
      (:Is%20Valid
        _)
      (:Is%20Not%20Valid
        (bind _returnvalue_2 (UserInterface|CreateWidget "/Game/03_su/WidgetBP/Pause.Pause_C"))
        (Variables|Default|SetPause%20Reference _returnvalue_2)))
    (Variables|/Script/Engine.PlayerController|SetbShowMouseCursor _returnvalue true)
    (Input|SetInputModeUIOnly _returnvalue (Variables|Default|GetPause%20Reference) "DoNotLock")
    (UserInterface|Viewport|AddtoViewport (Variables|Default|GetPause%20Reference) 0)))

(fn ConstructionScript)

(fn RemoveOldInputsfromBuffer
  (params (CharacterReference :type CPP%20Character%20Object%20Reference)))

(fn SetUpInputMappings
  (bind _returnvalue (Class|InputSettings|GetInputSettings))
  (for _array_element (Class|InputSettings|GetActionNames _returnvalue)
    (for _array_element_2 (Class|InputSettings|GetActionMappingbyName _returnvalue _array_element)
      (if (Utilities|String|Contains (Utilities|String|ToString(Name) (.ActionName (Utilities|Struct|BreakInputActionKeyMapping _array_element_2))) "P2")
        (bind _player2_reference (Variables|Default|GetPlayer2%20Reference)
          (:then
            (if (Utilities|String|Contains (Utilities|String|ToString(Name) (.ActionName (Utilities|Struct|BreakInputActionKeyMapping _array_element_2))) "Jump")
              (Class|CPPCharacter|AddtoInputMap _player2_reference (Utilities|String|ToString(Text) (Class|KismetInputLibrary|KeyGetDisplayName (.Key (Utilities|Struct|BreakInputActionKeyMapping _array_element_2)))) "E_Jump")
              (elif (Utilities|String|Contains (Utilities|String|ToString(Name) (.ActionName (Utilities|Struct|BreakInputActionKeyMapping _array_element_2))) "Crouch")
                (Class|CPPCharacter|AddtoInputMap _player2_reference (Utilities|String|ToString(Text) (Class|KismetInputLibrary|KeyGetDisplayName (.Key (Utilities|Struct|BreakInputActionKeyMapping _array_element_2)))) "E_Crouch")
                (elif (Utilities|String|Contains (Utilities|String|ToString(Name) (.ActionName (Utilities|Struct|BreakInputActionKeyMapping _array_element_2))) "L_Punch")
                  (Class|CPPCharacter|AddtoInputMap _player2_reference (Utilities|String|ToString(Text) (Class|KismetInputLibrary|KeyGetDisplayName (.Key (Utilities|Struct|BreakInputActionKeyMapping _array_element_2)))) "E_LeftPunch")
                  (elif (Utilities|String|Contains (Utilities|String|ToString(Name) (.ActionName (Utilities|Struct|BreakInputActionKeyMapping _array_element_2))) "R_Punch")
                    (Class|CPPCharacter|AddtoInputMap _player2_reference (Utilities|String|ToString(Text) (Class|KismetInputLibrary|KeyGetDisplayName (.Key (Utilities|Struct|BreakInputActionKeyMapping _array_element_2)))) "E_RightPunch")
                    (elif (Utilities|String|Contains (Utilities|String|ToString(Name) (.ActionName (Utilities|Struct|BreakInputActionKeyMapping _array_element_2))) "L_Kick")
                      (Class|CPPCharacter|AddtoInputMap _player2_reference (Utilities|String|ToString(Text) (Class|KismetInputLibrary|KeyGetDisplayName (.Key (Utilities|Struct|BreakInputActionKeyMapping _array_element_2)))) "E_LeftKick")
                      (elif (Utilities|String|Contains (Utilities|String|ToString(Name) (.ActionName (Utilities|Struct|BreakInputActionKeyMapping _array_element_2))) "R_Kick")
                        (Class|CPPCharacter|AddtoInputMap _player2_reference (Utilities|String|ToString(Text) (Class|KismetInputLibrary|KeyGetDisplayName (.Key (Utilities|Struct|BreakInputActionKeyMapping _array_element_2)))) "E_RightKick"))))))))
          (:else))
        (elif (Utilities|String|Contains (Utilities|String|ToString(Name) (.ActionName (Utilities|Struct|BreakInputActionKeyMapping _array_element_2))) "Jump")
          (Class|CPPCharacter|AddtoInputMap (Utilities|String|ToString(Text) (Class|KismetInputLibrary|KeyGetDisplayName (.Key (Utilities|Struct|BreakInputActionKeyMapping _array_element_2)))) "E_Jump")
          (elif (Utilities|String|Contains (Utilities|String|ToString(Name) (.ActionName (Utilities|Struct|BreakInputActionKeyMapping _array_element_2))) "Crouch")
            (Class|CPPCharacter|AddtoInputMap (Utilities|String|ToString(Text) (Class|KismetInputLibrary|KeyGetDisplayName (.Key (Utilities|Struct|BreakInputActionKeyMapping _array_element_2)))) "E_Crouch")
            (elif (Utilities|String|Contains (Utilities|String|ToString(Name) (.ActionName (Utilities|Struct|BreakInputActionKeyMapping _array_element_2))) "L_Punch")
              (Class|CPPCharacter|AddtoInputMap (Utilities|String|ToString(Text) (Class|KismetInputLibrary|KeyGetDisplayName (.Key (Utilities|Struct|BreakInputActionKeyMapping _array_element_2)))) "E_LeftPunch")
              (elif (Utilities|String|Contains (Utilities|String|ToString(Name) (.ActionName (Utilities|Struct|BreakInputActionKeyMapping _array_element_2))) "R_Punch")
                (Class|CPPCharacter|AddtoInputMap (Utilities|String|ToString(Text) (Class|KismetInputLibrary|KeyGetDisplayName (.Key (Utilities|Struct|BreakInputActionKeyMapping _array_element_2)))) "E_RightPunch")
                (elif (Utilities|String|Contains (Utilities|String|ToString(Name) (.ActionName (Utilities|Struct|BreakInputActionKeyMapping _array_element_2))) "L_Kick")
                  (Class|CPPCharacter|AddtoInputMap (Utilities|String|ToString(Text) (Class|KismetInputLibrary|KeyGetDisplayName (.Key (Utilities|Struct|BreakInputActionKeyMapping _array_element_2)))) "E_LeftKick")
                  (elif (Utilities|String|Contains (Utilities|String|ToString(Name) (.ActionName (Utilities|Struct|BreakInputActionKeyMapping _array_element_2))) "R_Kick")
                    (Class|CPPCharacter|AddtoInputMap (Utilities|String|ToString(Text) (Class|KismetInputLibrary|KeyGetDisplayName (.Key (Utilities|Struct|BreakInputActionKeyMapping _array_element_2)))) "E_RightKick"))))))))))
  (CallFunction|SetUpInputAxes))

(fn SetUpInputAxes
  (bind _returnvalue (Class|InputSettings|GetInputSettings))
  (for _array_element (Class|InputSettings|GetAxisNames _returnvalue)
    (for _array_element_2 (Class|InputSettings|GetAxisMappingbyName _returnvalue _array_element)
      (if (Utilities|String|Contains (Utilities|String|ToString(Name) (.AxisName (Utilities|Struct|BreakInputAxisKeyMapping _array_element_2))) "P2")
        (bind _player2_reference (Variables|Default|GetPlayer2%20Reference)
          (:then
            (if (Utilities|String|Contains (Utilities|String|ToString(Name) (.AxisName (Utilities|Struct|BreakInputAxisKeyMapping _array_element_2))) "MoveRight")
              (if (> (.Scale (Utilities|Struct|BreakInputAxisKeyMapping _array_element_2)) 0.0)
                (Class|CPPCharacter|AddtoInputMap _player2_reference (Utilities|String|ToString(Text) (Class|KismetInputLibrary|KeyGetDisplayName (.Key (Utilities|Struct|BreakInputAxisKeyMapping _array_element_2)))) "E_Forward")
                (else
                  (Class|CPPCharacter|AddtoInputMap _player2_reference (Utilities|String|ToString(Text) (Class|KismetInputLibrary|KeyGetDisplayName (.Key (Utilities|Struct|BreakInputAxisKeyMapping _array_element_2)))) "E_Backward")))))
          (:else))
        (elif (Utilities|String|Contains (Utilities|String|ToString(Name) (.AxisName (Utilities|Struct|BreakInputAxisKeyMapping _array_element_2))) "MoveRight")
          (if (> (.Scale (Utilities|Struct|BreakInputAxisKeyMapping _array_element_2)) 0.0)
            (Class|CPPCharacter|AddtoInputMap (Utilities|String|ToString(Text) (Class|KismetInputLibrary|KeyGetDisplayName (.Key (Utilities|Struct|BreakInputAxisKeyMapping _array_element_2)))) "E_Forward")
            (else
              (Class|CPPCharacter|AddtoInputMap (Utilities|String|ToString(Text) (Class|KismetInputLibrary|KeyGetDisplayName (.Key (Utilities|Struct|BreakInputAxisKeyMapping _array_element_2)))) "E_Backward")))))))
  (CallFunction|SetUpPlayerMappings))

(fn SetUpPlayerMappings
  (bind _returnvalue (Class|InputSettings|GetInputSettings))
  (for _array_element (Class|InputSettings|GetActionNames _returnvalue)
    (for _array_element_2 (Class|InputSettings|GetActionMappingbyName _returnvalue _array_element)
      (if (Utilities|String|Contains (Utilities|String|ToString(Name) (.ActionName (Utilities|Struct|BreakInputActionKeyMapping _array_element_2))) "P1")
        (Class|InputSettings|AddActionMapping _returnvalue (Utilities|Struct|MakeInputActionKeyMapping "AddToInputBuffer_P1" false false false false (.Key (Utilities|Struct|BreakInputActionKeyMapping _array_element_2))) true)
        (elif (Utilities|String|Contains (Utilities|String|ToString(Name) (.ActionName (Utilities|Struct|BreakInputActionKeyMapping _array_element_2))) "P2")
          (Class|InputSettings|AddActionMapping _returnvalue (Utilities|Struct|MakeInputActionKeyMapping "AddToInputBuffer_P2" false false false false (.Key (Utilities|Struct|BreakInputActionKeyMapping _array_element_2))) true))))))