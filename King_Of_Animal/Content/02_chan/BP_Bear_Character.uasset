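; Bear fighter character for a local two-player fighting game that also relays Player 2's movement and attack inputs to the game mode's Player2.
; On player lock-in, it scans input settings to build each player's key-to-move map, then adds buffer actions at runtime to action keys tagged P1 or P2.
; Those actions feed per-player timestamped input buffers, pruning stale entries before each add.
; Q or Escape opens the pause menu.
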(event EventBeginPlay
  (bind _asking_of_animal_game_mode (Utilities|Casting|CastToKing_Of_AnimalGameMode (Game|GetGameMode)))
  (Utilities|IsValid (Variables|/Script/King_Of_Animal.King_Of_AnimalGameMode|Getplayer2 _asking_of_animal_game_mode)
    (:Is%20Valid
      (Variables|Default|SetPlayer%202%20Reference (Variables|/Script/King_Of_Animal.King_Of_AnimalGameMode|Getplayer2 _asking_of_animal_game_mode)))))

(event EventNotifyPlayerLockedin
  (CallFunction|SetUpInputMappings))

(event Input|ActionEvents|InputActionJumpP2
  (params (Key :type Key%20Structure))
  (bind _player_2_reference (Variables|Default|GetPlayer%202%20Reference))
  (bind _player_2_reference_2 (Variables|Default|GetPlayer%202%20Reference))
  (:Pressed
    (Utilities|IsValid _player_2_reference_2
      (:Is%20Valid
        (Class|CPPCharacter|JumpP2 _player_2_reference_2))))
  (:Released
    (Utilities|IsValid _player_2_reference
      (:Is%20Valid
        (Class|CPPCharacter|StopJumpP2 _player_2_reference)))))

(event Input|ActionEvents|InputActionL_Punch_P2
  (params (Key :type Key%20Structure))
  (bind _player_2_reference (Variables|Default|GetPlayer%202%20Reference))
  (:Pressed
    (Utilities|IsValid _player_2_reference
      (:Is%20Valid
        (Class|CPPCharacter|LPunchP2 _player_2_reference)))))

(event Input|ActionEvents|InputActionUppercut_P2
  (params (Key :type Key%20Structure))
  (bind _player_2_reference (Variables|Default|GetPlayer%202%20Reference))
  (:Pressed
    (Utilities|IsValid _player_2_reference
      (:Is%20Valid
        (Class|CPPCharacter|UppercutP2 _player_2_reference)))))

(event Input|ActionEvents|InputActionR_Punch_P2
  (params (Key :type Key%20Structure))
  (bind _player_2_reference (Variables|Default|GetPlayer%202%20Reference))
  (:Pressed
    (Utilities|IsValid _player_2_reference
      (:Is%20Valid
        (Class|CPPCharacter|RPunchP2 _player_2_reference)))))

(event Input|ActionEvents|InputActionL_Kick_P2
  (params (Key :type Key%20Structure))
  (bind _player_2_reference (Variables|Default|GetPlayer%202%20Reference))
  (:Pressed
    (Utilities|IsValid _player_2_reference
      (:Is%20Valid
        (Class|CPPCharacter|LKickP2 _player_2_reference)))))

(event Input|ActionEvents|InputActionR_Kick_P2
  (params (Key :type Key%20Structure))
  (bind _player_2_reference (Variables|Default|GetPlayer%202%20Reference))
  (:Pressed
    (Utilities|IsValid _player_2_reference
      (:Is%20Valid
        (Class|CPPCharacter|RKickP2 _player_2_reference)))))

(event Input|ActionEvents|InputActionCrouch_P2
  (params (Key :type Key%20Structure))
  (bind _player_2_reference (Variables|Default|GetPlayer%202%20Reference))
  (bind _player_2_reference_2 (Variables|Default|GetPlayer%202%20Reference))
  (:Pressed
    (Utilities|IsValid _player_2_reference
      (:Is%20Valid
        (Class|CPPCharacter|StartCrouching _player_2_reference))))
  (:Released
    (Utilities|IsValid _player_2_reference_2
      (:Is%20Valid
        (Class|CPPCharacter|StopCrouching _player_2_reference_2)))))

(event Input|ActionEvents|InputActionUppercut_P2
  (params (Key :type Key%20Structure))
  (bind _player_2_reference (Variables|Default|GetPlayer%202%20Reference))
  (:Pressed
    (Utilities|IsValid _player_2_reference
      (:Is%20Valid
        (Class|CPPCharacter|UppercutP2 _player_2_reference)))))

(event Input|ActionEvents|InputActionExceptionalAttack_P2
  (params (Key :type Key%20Structure))
  (bind _player_2_reference (Variables|Default|GetPlayer%202%20Reference))
  (:Pressed
    (Utilities|IsValid _player_2_reference
      (:Is%20Valid
        (Class|CPPCharacter|StartExceptionalAttackP2 _player_2_reference)))))

(event Input|ActionEvents|InputActionAddToInputBuffer_P1
  (params (Key :type Key%20Structure))
  (bind _returnvalue (Class|KismetInputLibrary|KeyGetDisplayName Key))
  (bind _returnvalue_2 (Utilities|String|ToString(Text) _returnvalue))
  (:Pressed
    (CallFunction|RemoveOldInputsfromBuffer self)
    (Class|CPPCharacter|AddInputtoInputBuffer (Utilities|Struct|MakeInputInfo (.Value (Utilities|Map|Find (Variables|Default|GetinputToInputTypeMap) _returnvalue_2)) _returnvalue_2 (Utilities|Time|GetTimeSeconds) false))))

(event Input|ActionEvents|InputActionAddToInputBuffer_P2
  (params (Key :type Key%20Structure))
  (bind _returnvalue (Class|KismetInputLibrary|KeyGetDisplayName Key))
  (bind _player_2_reference (Variables|Default|GetPlayer%202%20Reference))
  (bind _returnvalue_2 (Utilities|String|ToString(Text) _returnvalue))
  (:Pressed
    (bind _player_2_reference_2 (Variables|Default|GetPlayer%202%20Reference)
      (:then
        (CallFunction|RemoveOldInputsfromBuffer _player_2_reference_2)
        (Class|CPPCharacter|AddInputtoInputBuffer _player_2_reference (Utilities|Struct|MakeInputInfo (.Value (Utilities|Map|Find (Variables|/Script/King_Of_Animal.CPP_Character|GetinputToInputTypeMap _player_2_reference) _returnvalue_2)) _returnvalue_2 (Utilities|Time|GetTimeSeconds) false)))
      (:else))))

(event Input|AxisEvents|InputAxisMoveRight_P2
  (params (AxisValue :type Float%20%28single-precision%29))
  (bind _player_2_reference (Variables|Default|GetPlayer%202%20Reference))
  (Utilities|IsValid _player_2_reference
    (:Is%20Valid
      (Class|CPPCharacter|MoveRightP2 _player_2_reference AxisValue))))

(event Input|KeyboardEvents|Escape
  (params (Key :type Key%20Structure))
  (bind _returnvalue (Game|GetPlayerController 0))
  ;[1 1 1] Pause Menu
  (:Pressed
    (Utilities|IsValid (Variables|Default|GetPause%20Reference)
      (:Is%20Valid
        _)
      (:Is%20Not%20Valid
        (bind _returnvalue_2 (UserInterface|CreateWidget "/Game/03_su/WidgetBP/Pause_UI.Pause_UI_C"))
        (Variables|Default|SetPause%20Reference _returnvalue_2)))
    (Variables|/Script/Engine.PlayerController|SetbShowMouseCursor _returnvalue true)
    (Input|SetInputModeUIOnly _returnvalue (Variables|Default|GetPause%20Reference) "DoNotLock")
    (UserInterface|Viewport|AddtoViewport (Variables|Default|GetPause%20Reference) 0)))

(event Input|KeyboardEvents|Q
  (params (Key :type Key%20Structure))
  (bind _returnvalue (Game|GetPlayerController 0))
  ;[1 1 1] Pause Menu
  (:Pressed
    (Utilities|IsValid (Variables|Default|GetPause%20Reference)
      (:Is%20Valid
        _)
      (:Is%20Not%20Valid
        (bind _returnvalue_2 (UserInterface|CreateWidget "/Game/03_su/WidgetBP/Pause_UI.Pause_UI_C"))
        (Variables|Default|SetPause%20Reference _returnvalue_2)))
    (Variables|/Script/Engine.PlayerController|SetbShowMouseCursor _returnvalue true)
    (Input|SetInputModeUIOnly _returnvalue (Variables|Default|GetPause%20Reference) "DoNotLock")
    (UserInterface|Viewport|AddtoViewport (Variables|Default|GetPause%20Reference) 0)))

(fn ConstructionScript)

(fn SetUpInputMappings
  (bind _returnvalue (Class|InputSettings|GetInputSettings))
  (for _array_element (Class|InputSettings|GetActionNames _returnvalue)
    (for _array_element_2 (Class|InputSettings|GetActionMappingbyName _returnvalue _array_element)
      (if (Utilities|String|Contains (Utilities|String|ToString(Name) (.ActionName (Utilities|Struct|BreakInputActionKeyMapping _array_element_2))) "P2")
        (bind _player_2_reference (Variables|Default|GetPlayer%202%20Reference)
          (:then
            (if (Utilities|String|Contains (Utilities|String|ToString(Name) (.ActionName (Utilities|Struct|BreakInputActionKeyMapping _array_element_2))) "Forward")
              (Class|CPPCharacter|AddtoInputMap _player_2_reference (Utilities|String|ToString(Text) (Class|KismetInputLibrary|KeyGetDisplayName (.Key (Utilities|Struct|BreakInputActionKeyMapping _array_element_2)))) "E_Forward")
              (elif (Utilities|String|Contains (Utilities|String|ToString(Name) (.ActionName (Utilities|Struct|BreakInputActionKeyMapping _array_element_2))) "Backward")
                (Class|CPPCharacter|AddtoInputMap _player_2_reference (Utilities|String|ToString(Text) (Class|KismetInputLibrary|KeyGetDisplayName (.Key (Utilities|Struct|BreakInputActionKeyMapping _array_element_2)))) "E_Backward")
                (elif (Utilities|String|Contains (Utilities|String|ToString(Name) (.ActionName (Utilities|Struct|BreakInputActionKeyMapping _array_element_2))) "Jump")
                  (Class|CPPCharacter|AddtoInputMap _player_2_reference (Utilities|String|ToString(Text) (Class|KismetInputLibrary|KeyGetDisplayName (.Key (Utilities|Struct|BreakInputActionKeyMapping _array_element_2)))) "E_Jump")
                  (elif (Utilities|String|Contains (Utilities|String|ToString(Name) (.ActionName (Utilities|Struct|BreakInputActionKeyMapping _array_element_2))) "Crouch")
                    (Class|CPPCharacter|AddtoInputMap _player_2_reference (Utilities|String|ToString(Text) (Class|KismetInputLibrary|KeyGetDisplayName (.Key (Utilities|Struct|BreakInputActionKeyMapping _array_element_2)))) "E_Crouch")
                    (elif (Utilities|String|Contains (Utilities|String|ToString(Name) (.ActionName (Utilities|Struct|BreakInputActionKeyMapping _array_element_2))) "L_Punch")
                      (Class|CPPCharacter|AddtoInputMap _player_2_reference (Utilities|String|ToString(Text) (Class|KismetInputLibrary|KeyGetDisplayName (.Key (Utilities|Struct|BreakInputActionKeyMapping _array_element_2)))) "E_LeftPunch")
                      (elif (Utilities|String|Contains (Utilities|String|ToString(Name) (.ActionName (Utilities|Struct|BreakInputActionKeyMapping _array_element_2))) "R_Punch")
                        (Class|CPPCharacter|AddtoInputMap _player_2_reference (Utilities|String|ToString(Text) (Class|KismetInputLibrary|KeyGetDisplayName (.Key (Utilities|Struct|BreakInputActionKeyMapping _array_element_2)))) "E_RightPunch")
                        (elif (Utilities|String|Contains (Utilities|String|ToString(Name) (.ActionName (Utilities|Struct|BreakInputActionKeyMapping _array_element_2))) "L_Kick")
                          (Class|CPPCharacter|AddtoInputMap _player_2_reference (Utilities|String|ToString(Text) (Class|KismetInputLibrary|KeyGetDisplayName (.Key (Utilities|Struct|BreakInputActionKeyMapping _array_element_2)))) "E_LeftKick")
                          (elif (Utilities|String|Contains (Utilities|String|ToString(Name) (.ActionName (Utilities|Struct|BreakInputActionKeyMapping _array_element_2))) "R_Kick")
                            (Class|CPPCharacter|AddtoInputMap _player_2_reference (Utilities|String|ToString(Text) (Class|KismetInputLibrary|KeyGetDisplayName (.Key (Utilities|Struct|BreakInputActionKeyMapping _array_element_2)))) "E_RightKick"))))))))))
          (:else))
        (elif (Utilities|String|Contains (Utilities|String|ToString(Name) (.ActionName (Utilities|Struct|BreakInputActionKeyMapping _array_element_2))) "Forward")
          (Class|CPPCharacter|AddtoInputMap (Utilities|String|ToString(Text) (Class|KismetInputLibrary|KeyGetDisplayName (.Key (Utilities|Struct|BreakInputActionKeyMapping _array_element_2)))) "E_Forward")
          (elif (Utilities|String|Contains (Utilities|String|ToString(Name) (.ActionName (Utilities|Struct|BreakInputActionKeyMapping _array_element_2))) "Backward")
            (Class|CPPCharacter|AddtoInputMap (Utilities|String|ToString(Text) (Class|KismetInputLibrary|KeyGetDisplayName (.Key (Utilities|Struct|BreakInputActionKeyMapping _array_element_2)))) "E_Backward")
            (elif (Utilities|String|Contains (Utilities|String|ToString(Name) (.ActionName (Utilities|Struct|BreakInputActionKeyMapping _array_element_2))) "Jump")
              (Class|CPPCharacter|AddtoInputMap (Utilities|String|ToString(Text) (Class|KismetInputLibrary|KeyGetDisplayName (.Key (Utilities|Struct|BreakInputActionKeyMapping _array_element_2)))) "E_Jump")
              (elif (Utilities|String|Contains (Utilities|String|ToString(Name) (.ActionName (Utilities|Struct|BreakInputActionKeyMapping _array_element_2))) "Crouch")
                (Class|CPPCharacter|AddtoInputMap (Utilities|String|ToString(Text) (Class|KismetInputLibrary|KeyGetDisplayName (.Key (Utilities|Struct|BreakInputActionKeyMapping _array_element_2)))) "E_Crouch")
                (elif (Utilities|String|Contains (Utilities|String|ToString(Name) (.ActionName (Utilities|Struct|BreakInputActionKeyMapping _array_element_2))) "L_Punch")
                  (Class|CPPCharacter|AddtoInputMap (Utilities|String|ToString(Text) (Class|KismetInputLibrary|KeyGetDisplayName (.Key (Utilities|Struct|BreakInputActionKeyMapping _array_element_2)))) "E_LeftPunch")
                  (elif (Utilities|String|Contains (Utilities|String|ToString(Name) (.ActionName (Utilities|Struct|BreakInputActionKeyMapping _array_element_2))) "R_Punch")
                    (Class|CPPCharacter|AddtoInputMap (Utilities|String|ToString(Text) (Class|KismetInputLibrary|KeyGetDisplayName (.Key (Utilities|Struct|BreakInputActionKeyMapping _array_element_2)))) "E_RightPunch")
                    (elif (Utilities|String|Contains (Utilities|String|ToString(Name) (.ActionName (Utilities|Struct|BreakInputActionKeyMapping _array_element_2))) "L_Kick")
                      (Class|CPPCharacter|AddtoInputMap (Utilities|String|ToString(Text) (Class|KismetInputLibrary|KeyGetDisplayName (.Key (Utilities|Struct|BreakInputActionKeyMapping _array_element_2)))) "E_LeftKick")
                      (elif (Utilities|String|Contains (Utilities|String|ToString(Name) (.ActionName (Utilities|Struct|BreakInputActionKeyMapping _array_element_2))) "R_Kick")
                        (Class|CPPCharacter|AddtoInputMap (Utilities|String|ToString(Text) (Class|KismetInputLibrary|KeyGetDisplayName (.Key (Utilities|Struct|BreakInputActionKeyMapping _array_element_2)))) "E_RightKick"))))))))))))
  (CallFunction|SetUpInputAxes))

(fn RemoveOldInputsfromBuffer
  (params (CharacterReference :type CPP%20Character%20Object%20Reference))
  (bind _indicies_to_remove (LocalVariables|GetIndicies%20to%20Remove))
  (bind _returnvalue (Utilities|Array|LastIndex _indicies_to_remove))
  (for _index (range 0 (Utilities|Array|LastIndex (Variables|/Script/King_Of_Animal.CPP_Character|GetinputBuffer CharacterReference)))
    (if (< (.timeStamp (Utilities|Struct|BreakInputInfo (Utilities|Array|Get(acopy) (Variables|/Script/King_Of_Animal.CPP_Character|GetinputBuffer CharacterReference) _index))) (- (Utilities|Time|GetTimeSeconds) 0.2))
      (Utilities|Array|AddUnique (LocalVariables|GetIndicies%20to%20Remove) _index)))
  (for _index_2 (range 0 _returnvalue)
    (Utilities|Array|RemoveIndex (Variables|/Script/King_Of_Animal.CPP_Character|GetinputBuffer CharacterReference) (- _returnvalue _index_2)))
  (Utilities|Array|Clear _indicies_to_remove))

(fn SetUpInputAxes
  (bind _returnvalue (Class|InputSettings|GetInputSettings))
  (for _array_element (Class|InputSettings|GetAxisNames _returnvalue)
    (for _array_element_2 (Class|InputSettings|GetAxisMappingbyName _returnvalue _array_element)
      (if (Utilities|String|Contains (Utilities|String|ToString(Name) (.AxisName (Utilities|Struct|BreakInputAxisKeyMapping _array_element_2))) "P2")
        (bind _player_2_reference (Variables|Default|GetPlayer%202%20Reference)
          (:then
            (if (Utilities|String|Contains (Utilities|String|ToString(Name) (.AxisName (Utilities|Struct|BreakInputAxisKeyMapping _array_element_2))) "MoveRight")
              (if (> (.Scale (Utilities|Struct|BreakInputAxisKeyMapping _array_element_2)) 0.0)
                (Class|CPPCharacter|AddtoInputMap _player_2_reference (Utilities|String|ToString(Text) (Class|KismetInputLibrary|KeyGetDisplayName (.Key (Utilities|Struct|BreakInputAxisKeyMapping _array_element_2)))) "E_Forward")
                (else
                  (Class|CPPCharacter|AddtoInputMap _player_2_reference (Utilities|String|ToString(Text) (Class|KismetInputLibrary|KeyGetDisplayName (.Key (Utilities|Struct|BreakInputAxisKeyMapping _array_element_2)))) "E_Backward")))))
          (:else))
        (elif (Utilities|String|Contains (Utilities|String|ToString(Name) (.AxisName (Utilities|Struct|BreakInputAxisKeyMapping _array_element_2))) "MoveRight")
          (if (> (.Scale (Utilities|Struct|BreakInputAxisKeyMapping _array_element_2)) 0.0)
            (Class|CPPCharacter|AddtoInputMap (Utilities|String|ToString(Text) (Class|KismetInputLibrary|KeyGetDisplayName (.Key (Utilities|Struct|BreakInputAxisKeyMapping _array_element_2)))) "E_Forward")
            (else
              (Class|CPPCharacter|AddtoInputMap (Utilities|String|ToString(Text) (Class|KismetInputLibrary|KeyGetDisplayName (.Key (Utilities|Struct|BreakInputAxisKeyMapping _array_element_2)))) "E_Backward")))))))
  (CallFunction|SetUpPlayerMappings))

(fn SetUpPlayerMappings
  (bind _returnvalue (Class|InputSettings|GetInputSettings))
  (for _array_element (Class|InputSettings|GetActionNames _returnvalue)
    (for _array_element_2 (Class|InputSettings|GetActionMappingbyName _returnvalue _array_element)
      (if (Utilities|String|Contains (Utilities|String|ToString(Name) (.ActionName (Utilities|Struct|BreakInputActionKeyMapping _array_element_2))) "P1")
        (Class|InputSettings|AddActionMapping _returnvalue (Utilities|Struct|MakeInputActionKeyMapping "AddToInputBuffer_P1" false false false false (.Key (Utilities|Struct|BreakInputActionKeyMapping _array_element_2))) true)
        (elif (Utilities|String|Contains (Utilities|String|ToString(Name) (.ActionName (Utilities|Struct|BreakInputActionKeyMapping _array_element_2))) "P2")
          (Class|InputSettings|AddActionMapping _returnvalue (Utilities|Struct|MakeInputActionKeyMapping "AddToInputBuffer_P2" false false false false (.Key (Utilities|Struct|BreakInputActionKeyMapping _array_element_2))) true))))))