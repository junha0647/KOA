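; Donkey character Blueprint that relays second-player input for a fighting game.
; On BeginPlay it caches the Player2 reference from King_Of_AnimalGameMode.
; Its P2 input events for horizontal movement, jump press and release, and left and right punches and kicks forward to that reference after a validity check.
; It holds no movement or attack logic for itself in these graphs.
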(event EventBeginPlay
  (bind _asking_of_animal_game_mode (Utilities|Casting|CastToKing_Of_AnimalGameMode (Game|GetGameMode)))
  (Utilities|IsValid (Variables|/Script/King_Of_Animal.King_Of_AnimalGameMode|Getplayer2 _asking_of_animal_game_mode)
    (:Is%20Valid
      (Variables|Default|SetPlayer2%20Reference (Variables|/Script/King_Of_Animal.King_Of_AnimalGameMode|Getplayer2 _asking_of_animal_game_mode)))))

(event Collision|EventActorBeginOverlap
  (params (OtherActor :type Actor%20Object%20Reference)))

(event EventTick
  (params (DeltaSeconds :type Float%20%28single-precision%29)))

(event Input|ActionEvents|InputActionJumpP2
  (params (Key :type Key%20Structure :default "None"))
  (bind _player2_reference (Variables|Default|GetPlayer2%20Reference))
  (bind _player2_reference_2 (Variables|Default|GetPlayer2%20Reference))
  (:Pressed
    (Utilities|IsValid _player2_reference
      (:Is%20Valid
        (Class|CPPCharacter|JumpP2 _player2_reference))))
  (:Released
    (Utilities|IsValid _player2_reference_2
      (:Is%20Valid
        (Class|CPPCharacter|StopJumpP2 _player2_reference_2)))))

(event Input|ActionEvents|InputActionL_Punch_P2
  (params (Key :type Key%20Structure :default "None"))
  (bind _player2_reference (Variables|Default|GetPlayer2%20Reference))
  (:Pressed
    (Utilities|IsValid _player2_reference
      (:Is%20Valid
        (Class|CPPCharacter|LPunchP2 _player2_reference)))))

(event Input|ActionEvents|InputActionR_Punch_P2
  (params (Key :type Key%20Structure :default "None"))
  (bind _player2_reference (Variables|Default|GetPlayer2%20Reference))
  (:Pressed
    (Utilities|IsValid _player2_reference
      (:Is%20Valid
        (Class|CPPCharacter|RPunchP2 _player2_reference)))))

(event Input|ActionEvents|InputActionL_Kick_P2
  (params (Key :type Key%20Structure :default "None"))
  (bind _player2_reference (Variables|Default|GetPlayer2%20Reference))
  (:Pressed
    (Utilities|IsValid _player2_reference
      (:Is%20Valid
        (Class|CPPCharacter|LKickP2 _player2_reference)))))

(event Input|ActionEvents|InputActionR_Kick_P2
  (params (Key :type Key%20Structure :default "None"))
  (bind _player2_reference (Variables|Default|GetPlayer2%20Reference))
  (:Pressed
    (Utilities|IsValid _player2_reference
      (:Is%20Valid
        (Class|CPPCharacter|RKickP2 _player2_reference)))))

(event Input|AxisEvents|InputAxisMoveRight_P2
  (params (AxisValue :type Float%20%28single-precision%29))
  (bind _player2_reference (Variables|Default|GetPlayer2%20Reference))
  (Utilities|IsValid _player2_reference
    (:Is%20Valid
      (Class|CPPCharacter|MoveRightP2 _player2_reference AxisValue))))

(fn ConstructionScript)