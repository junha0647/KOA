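; Game mode for a two-character versus game that spawns and possesses both fighters at the tagged player starts.
; On BeginPlay, P1 goes to the first player controller and P2 to a newly spawned BasePlayerController.
; DetermineCharacterClass picks Donkey or Elephant from the game instance's single CharacterClass, so both players share the choice.
; It then links the two as opponents, flips Player2 and shows the health widget.
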(event EventBeginPlay
  (bind _player1 (Variables|Default|Getplayer1))
  (bind _player2 (Variables|Default|Getplayer2))
  (bind _outactors (Actor|GetAllActorsOfClass "/Script/Engine.PlayerStart"))
  (for _array_element _outactors
    (CallFunction|SpawnPlayers _array_element))
  (if (Utilities|IsValid (Variables|Default|Getplayer1))
    (if (Utilities|IsValid (Variables|Default|Getplayer2))
      (Variables|/Script/King_Of_Animal.CPP_Character|Setopponent _player1 _player2)
      (Variables|/Script/King_Of_Animal.CPP_Character|Setopponent _player2 _player1)
      (Variables|/Script/King_Of_Animal.CPP_Character|SetisFlipped _player2 true)
      (bind _returnvalue (UserInterface|CreateWidget "/Game/03_su/WBP_Health.WBP_Health_C" (Game|GetPlayerController 0)))
      (UserInterface|Viewport|AddtoViewport _returnvalue 0))))

(event EventTick
  (params (DeltaSeconds :type Float%20%28single-precision%29)))

(fn ConstructionScript)

(fn SpawnPlayers
  (params (Object :type Actor%20Object%20Reference))
  (bind _returnvalue (Transformation|GetActorTransform Object))
  (bind _asplayer_start (Utilities|Casting|CastToPlayerStart Object))
  (if (Utilities|Name|Equal(Name) "P1" (Variables|/Script/Engine.PlayerStart|GetPlayerStartTag _asplayer_start))
    (bind _character_reference (CallFunction|DetermineCharacterClass (Transformation|GetActorTransform Object) Object))
    (Variables|Default|Setplayer1 _character_reference)
    (Pawn|Possess (Game|GetPlayerController 0) _character_reference)
    (elif (Utilities|Name|Equal(Name) (Variables|/Script/Engine.PlayerStart|GetPlayerStartTag _asplayer_start) "P2")
      (bind _returnvalue_2 (Game|SpawnActorfromClass "/Script/King_Of_Animal.BasePlayerController" _returnvalue "Undefined" 0 0))
      (bind _character_reference_2 (CallFunction|DetermineCharacterClass _returnvalue Object))
      (Variables|Default|Setplayer2 _character_reference_2)
      (Pawn|Possess _returnvalue_2 _character_reference_2))))

(fn DetermineCharacterClass
  (params (Transform :type Transform) (Actor :type Actor%20Object%20Reference))
  (bind _asbase_game_instance (Utilities|Casting|CastToBaseGameInstance (Game|GetGameInstance)))
  (switch Utilities|FlowControl|Switch|SwitchonECharacterClass (Variables|/Script/King_Of_Animal.BaseGameInstance|GetcharacterClass _asbase_game_instance)
    (:VE_Default
      (bind _returnvalue (Game|SpawnActorfromClass "/Game/02_chan/BP_Donkey_Character.BP_Donkey_Character_C" Transform "Undefined" Actor 0))
      (return _returnvalue))
    (:VE_Mutant
      (bind _returnvalue_2 (Game|SpawnActorfromClass "/Game/02_chan/BP_Elephant_Character.BP_Elephant_Character_C" Transform "Undefined" Actor 0))
      (return _returnvalue_2))))